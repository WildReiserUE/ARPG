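; Static-mesh pickup class for the ARPG inventory's pickup system, providing highlight and prompt feedback.
; SetOutlineEnabled stores the outline state in BPNameVisibility and toggles the mesh's custom depth rendering to match.
; When given a valid interact key, it sets that key's display name on the BP_DisplayName widget, flagged to clear when disabling.
; It then shows or hides the pickup widget; the event graph has no active logic.
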(event EventBeginPlay
  (|CallParentFunction) ; This node is disabled and will not be called.\nDrag off pins to build functionality.
)

(event Collision|EventActorBeginOverlap
  (params (OtherActor :type Actor%20Object%20Reference)))

(event EventTick
  (params (DeltaSeconds :type Float%20%28single-precision%29)))

(fn ConstructionScript
  (|CallParentFunction))

(fn SetOutlineEnabled
  (params (Enabled :type Boolean) (InteractKey :type Key%20Structure) (CalledFrom :type Actor%20Object%20Reference))
  (bind _nonekey (LocalVariables|GetNoneKey))
  (bind _returnvalue (== InteractKey _nonekey))
  (bind _output_get (Variables|/Game/ARPG/Blueprints/Components/BP_NameVisibility.BP_NameVisibility_C|SetOutlineOn (Variables|Default|GetBP_NameVisibility) Enabled))
  (Rendering|SetRenderCustomDepth (Variables|Default|GetStaticMesh) _output_get)
  (Utilities|FlowControl|Sequence
    (:then_0
      (if (not _returnvalue)
        (bind _asbp_display_name (Utilities|Casting|CastToBP_DisplayName (UserInterface|GetUserWidgetObject (Variables|Default|GetWidget))))
        (Default|SetInteractKey _asbp_display_name (Class|KismetInputLibrary|KeyGetDisplayName InteractKey) (or _returnvalue (not Enabled)))))
    (:then_1
      (CallFunction|ShowPickupWidget Enabled))
    (:then_2
      (return Enabled))))