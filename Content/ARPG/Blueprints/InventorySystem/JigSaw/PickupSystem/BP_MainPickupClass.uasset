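; Base item pickup actor for the ARPG inventory system that players can highlight and interact with to request a pickup.
; On BeginPlay the server initializes PickupComponent with optional random stats and count override, then the name widget shows item name, count and rarity color.
; Highlighting toggles custom-depth outline and an item info widget with mods and interact key.
; Interface functions expose physics, equipped state and outline color, with most combat and AI queries stubbed.
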(event EventBeginPlay
  (bind _pickupcomponent (Variables|Default|GetPickupComponent))
  ;[1 1 1] BEGIN PLAY
  (Utilities|FlowControl|Sequence
    (:then_0
      (Utilities|FlowControl|Sequence
        (:then_0
          (Networking|SwitchHasAuthority
            (:Authority
              (Default|Initialize (Variables|Default|GetPickupComponent) (Variables|Replication|GetSetRandomStats) (Variables|Replication|GetRandomStats)))))
        (:then_1
          (if (> (Variables|Replication|GetNewCount) -1)
            (Default|UpdateCount (Variables|Default|GetPickupComponent) (Variables|Replication|GetNewCount))))))
    (:then_1
      (bind _asbp_display_name (Utilities|Casting|CastToBP_DisplayName (UserInterface|GetUserWidgetObject (Variables|Default|GetWidget))))
      (Default|UpdateName _asbp_display_name (Default|GetItemNameCount _pickupcomponent) (Default|GetRarityColor _pickupcomponent)))))

(event EventSetPickupPhysicsEnabled
  (params (Enable? :type Boolean))
  ;[1 1 1] Interface events
  (Physics|SetSimulatePhysics (Variables|Default|GetBox) Enable?))

(event EventSetEquipped
  (params (Equipped :type Boolean))
  ;[1 1 1] Interface events
  (Variables|/Game/ARPG/Blueprints/InventorySystem/JigSaw/PickupSystem/BP_PickupComponent.BP_PickupComponent_C|SetEquipped (Variables|Default|GetPickupComponent) Equipped))

(event EventExecuteInteract
  (params (CharacterRef :type Actor%20Object%20Reference) (Comp :type BP%20Inventory%20Component%20Object%20Reference))
  ;[1 1 1] When interacted with
  (Default|RequestPickup Comp self))

(fn ConstructionScript
  (Variables|/Game/ARPG/Blueprints/InventorySystem/JigSaw/PickupSystem/BP_PickupComponent.BP_PickupComponent_C|SetRandomStatsManager (Variables|Default|GetPickupComponent) (Variables|Default|GetBP_RandomStatsManager))
  (Variables|/Game/ARPG/Blueprints/Components/BP_NameVisibility.BP_NameVisibility_C|SetWidget (Variables|Default|GetBP_NameVisibility) (Variables|Default|GetWidget)))

(fn GetMesh
  (return 0))

(fn GetMeshComponent
  (return (Variables|Default|GetSkeletalMesh) true))

(fn ShowPickupWidget
  (params (Enabled :type Boolean))
  (bind _pickupcomponent (Variables|Default|GetPickupComponent))
  (bind _asbp_display_name (Utilities|Casting|CastToBP_DisplayName (UserInterface|GetUserWidgetObject (Variables|Default|GetWidget))))
  (if Enabled
    (Class|WidgetComponent|SetPivot (Variables|Default|GetWidget) (Math|Vector2D|MakeVector2D 0.5 1.1))
    (Default|CreatePickupWidget _asbp_display_name (Default|GetInfo _pickupcomponent) (Default|GetItemMods _pickupcomponent) self)
    (else
      (Default|RemovePickupWidget _asbp_display_name)
      (Class|WidgetComponent|SetPivot (Variables|Default|GetWidget) (Math|Vector2D|MakeVector2D 0.5 1.5)))))

(fn CanbeDamagedbyPlayer?
  (return false))

(fn CanInteract?
  (return true 0.0))

(fn GetAcceptableDistance
  (return 1e+02))

(fn GetActorName
  (return ""))

(fn GetAIBehavior
  (return "NewEnumerator3"))

(fn GetAIHostility
  (return "NewEnumerator3"))

(fn GetBountyExp
  (return 0.0))

(fn GetOutlineColor
  (bind _pickupcomponent (Variables|Default|GetPickupComponent))
  (return (Math|Color|SelectColor "(R=0.000000,G=0.675999,B=1.000000,A=1.000000)" (Default|GetRarityColor _pickupcomponent) (Utilities|Enum|Equal(Enum) (Default|GetRarity _pickupcomponent) "NewEnumerator0"))))

(fn GetPickupComponent
  (return (Variables|Default|GetPickupComponent)))

(fn GetSkeletalAsset
  (return 0))

(fn OnBeginInteract
  (return false))

(fn OnEndInteract
  (return false))

(fn SetHostility
  (params (NewHostility :type E_AIHostilityType%20Enum :default "NewEnumerator3"))
  (return false))

(fn SetHostilityColor
  (params (IsHostile :type Boolean) (IsParty? :type Boolean) (IsGuild? :type Boolean))
  (return false))

(fn SetOutlineEnabled
  (params (Enabled :type Boolean) (InteractKey :type Key%20Structure) (CalledFrom :type Actor%20Object%20Reference))
  (bind _nonekey (LocalVariables|GetNoneKey))
  (bind _returnvalue (== InteractKey _nonekey))
  (Variables|/Game/ARPG/Blueprints/Components/BP_NameVisibility.BP_NameVisibility_C|SetOutlineOn (Variables|Default|GetBP_NameVisibility) Enabled)
  (Rendering|SetRenderCustomDepth (Variables|Default|GetSkeletalMesh) Enabled)
  (Utilities|FlowControl|Sequence
    (:then_0
      (if (not _returnvalue)
        (bind _asbp_display_name (Utilities|Casting|CastToBP_DisplayName (UserInterface|GetUserWidgetObject (Variables|Default|GetWidget))))
        (Default|SetInteractKey _asbp_display_name (Class|KismetInputLibrary|KeyGetDisplayName InteractKey) (or _returnvalue (not Enabled)))))
    (:then_1
      (CallFunction|ShowPickupWidget Enabled))
    (:then_2
      (return Enabled))))