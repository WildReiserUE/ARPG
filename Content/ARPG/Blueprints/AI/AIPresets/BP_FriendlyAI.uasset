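; BP_FriendlyAI is an AI character preset for an ally of the first player, shown with a green outline color.
; On BeginPlay, the authority retries every 0.2 seconds until player controller 0 and its controlled pawn are valid.
; It then registers that pawn as the friendly actor and sets the AI's hostility.
; The construction script makes armor, pants and head meshes follow the main mesh via master pose.
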(event EventBeginPlay
  (bind _returnvalue (Game|GetPlayerController 0))
  ;[1 1 1] Set friendly AI to follow a player, Hostility = player, Behavior = Aggressive
  (|CallParentFunction)
  (Networking|SwitchHasAuthority
    (:Authority
      (Utilities|IsValid _returnvalue :!label _label
        (:Is%20Valid
          (bind _actorref (Class|BPARPGControllerInterface|GetControlledPawnRef(Message) _returnvalue :!label _label_2))
          (Utilities|IsValid _actorref
            (:Is%20Valid
              (CallFunction|SetFriendlyActor _actorref)
              (CallFunction|SetHostility "NewEnumerator0"))
            (:Is%20Not%20Valid
              (Utilities|FlowControl|Delay 0.2)
              (goto _label_2))))
        (:Is%20Not%20Valid
          (Utilities|FlowControl|Delay 0.2)
          (goto _label))))))

(fn ConstructionScript
  (|CallParentFunction)
  (Class|SkinnedMeshComponent|SetMasterPoseComponent (Variables|Default|GetArmor_0) (Variables|Character|GetMesh) false))

(fn GetOutlineColor
  (return "(R=0.000000,G=1.000000,B=0.000000,A=1.000000)"))