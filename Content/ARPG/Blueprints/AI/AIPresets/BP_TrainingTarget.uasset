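; BP_TrainingTarget is an AI preset for a training target that replaces itself with a new copy after death.
; Its construction script caches the actor's transform in DefaultT.
; When OnAIDeathDestroyed fires, it runs the parent logic, then spawns its own class at that transform, adjusting for collisions but always spawning.
; OnAIDeath only forwards to the parent.
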(fn ConstructionScript
  (|CallParentFunction)
  (Variables|Default|SetDefaultT (Transformation|GetActorTransform)))

(fn OnAIDeath
  (|CallParentFunction))

(fn OnAIDeathDestroyed
  (|CallParentFunction)
  (Game|SpawnActorfromClass (Utilities|GetClass self) (Variables|Default|GetDefaultT) "AdjustIfPossibleButAlwaysSpawn" 0 "0.000000,0.000000,0.000000" false false 0 0))