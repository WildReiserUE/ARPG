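; BP_AIRespawner is a short-lived, server-side timer actor that respawns an AI through its home actor.
; On BeginPlay with authority, it waits a random delay within the RespawnTime range, then asks a valid AIHomeRef to respawn the AIClassToSpawn class.
; It destroys itself afterwards, whether or not the home reference was valid.
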(event EventBeginPlay
  (bind _respawntime (Variables|Default|GetRespawnTime))
  (bind _aihomeref (Variables|Default|GetAIHomeRef))
  (Networking|SwitchHasAuthority
    (:Authority
      (bind _output_get (Variables|Default|Setdur (Math|Random|RandomFloatinRange (.x _respawntime) (.y _respawntime))))
      (Utilities|FlowControl|Delay _output_get)
      (Utilities|FlowControl|Sequence
        (:then_0
          (Utilities|IsValid _aihomeref
            (:Is%20Valid
              (Default|RespawnerRespawnAI _aihomeref (Variables|Default|GetAIClassToSpawn)))))
        (:then_1
          (Actor|DestroyActor))))))

(fn ConstructionScript)