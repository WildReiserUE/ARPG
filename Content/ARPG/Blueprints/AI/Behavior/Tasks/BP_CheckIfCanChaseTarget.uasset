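; Behavior tree task that, going by its name, checks whether the AI can chase its enemy relative to a home location.
; On execute it caches the enemy, home location and home radius from the Blackboard.
; On tick it finishes, succeeding only if neither target nor pawn is any distance from home.
; Both distance tests compare against zero, leaving the cached radius unused.
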(event EventReceiveExecuteAI
  (params (OwnerController :type AI%20Controller%20Object%20Reference) (ControlledPawn :type Pawn%20Object%20Reference))
  (Variables|Default|SetTarget (AI|BehaviorTree|GetBlackboardValueasActor (Variables|Default|GetEnemy)))
  (Variables|Default|SetHomeLoc (Class|BTFunctionLibrary|GetBlackboardValueasVector (Variables|Default|GetHomeLocation)))
  (Variables|Default|SetRaduis (Class|BTFunctionLibrary|GetBlackboardValueasFloat (Variables|Default|GetHomeRaduis))))

(event EventReceiveTickAI
  (params (OwnerController :type AI%20Controller%20Object%20Reference) (ControlledPawn :type Pawn%20Object%20Reference) (DeltaSeconds :type Float%20%28single-precision%29))
  (AI|BehaviorTree|FinishExecute (not (or (> (Math|Vector|VectorLength (- (Transformation|GetActorLocation (Variables|Default|GetTarget)) (Variables|Default|GetHomeLoc))) 0.0) (> (Math|Vector|VectorLength (- (Transformation|GetActorLocation ControlledPawn) (Variables|Default|GetHomeLoc))) 0.0)))))