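; Behavior tree service that decides each tick whether an AI may chase its Enemy, writing the CanChase blackboard key.
; Home is the Friendly actor's location if valid, otherwise HomeLocation; chasing requires both pawn and target within twice HomeRaduis of it.
; When the enemy becomes invalid, it clears CanChase and, if it was just chasing, sets UseLastKnowLoc by whether the last known enemy location is in that range.
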(event EventReceiveTickAI
  (params (OwnerController :type AI%20Controller%20Object%20Reference) (ControlledPawn :type Pawn%20Object%20Reference) (DeltaSeconds :type Float%20%28single-precision%29))
  (bind _friendly (Variables|Default|GetFriendly))
  (bind _returnvalue (AI|BehaviorTree|GetBlackboardValueasActor _friendly))
  (Variables|Default|SetControlled%20Pawn ControlledPawn)
  (Variables|Default|SetTarget (AI|BehaviorTree|GetBlackboardValueasActor (Variables|Default|GetEnemy)))
  (Utilities|IsValid (Variables|Default|GetTarget)
    (:Is%20Valid
      (Variables|Default|SetIsChasing? true)
      (Utilities|IsValid _returnvalue
        (:Is%20Valid
          (Variables|Default|SetHomeLoc (Transformation|GetActorLocation _returnvalue)))
        (:Is%20Not%20Valid
          (Variables|Default|SetHomeLoc (Class|BTFunctionLibrary|GetBlackboardValueasVector (Variables|Default|GetHomeLocation)))))
      (Variables|Default|SetRaduis (Class|BTFunctionLibrary|GetBlackboardValueasFloat (Variables|Default|GetHomeRaduis)))
      ;[1 1 1] Can't chase if AI ts too far from home or target is outside AI home
      (bind _output_get (Variables|Default|SetCanC (not (or (> (Math|Vector|VectorLength (- (Transformation|GetActorLocation (Variables|Default|GetTarget)) (Variables|Default|GetHomeLoc))) (* (Variables|Default|GetRaduis) 2.0)) (> (Math|Vector|VectorLength (- (Transformation|GetActorLocation (Variables|Default|GetControlled%20Pawn)) (Variables|Default|GetHomeLoc))) (* (Variables|Default|GetRaduis) 2.0))))))
      (Class|BTFunctionLibrary|SetBlackboardValueasBool (Variables|Default|GetCanChase) _output_get))
    (:Is%20Not%20Valid
      (Class|BTFunctionLibrary|SetBlackboardValueasBool (Variables|Default|GetCanChase) false)
      (Utilities|FlowControl|Sequence
        (:then_0
          (if (and (Variables|Default|GetIsChasing?) (Variables|Default|GetCanC))
            (Class|BTFunctionLibrary|SetBlackboardValueasBool (Variables|Default|GetUseLastKnowLoc) (not (> (Math|Vector|VectorLength (- (Class|BTFunctionLibrary|GetBlackboardValueasVector (Variables|Default|GetLastKnowEnemyLoc)) (Variables|Default|GetHomeLoc))) (* (Variables|Default|GetRaduis) 2.0))))))
        (:then_1
          (Variables|Default|SetIsChasing? false))))))