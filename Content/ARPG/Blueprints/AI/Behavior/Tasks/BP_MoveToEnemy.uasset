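; Behavior tree task that moves an AI pawn to the enemy actor stored in the blackboard.
; On execute it orients rotation to movement and runs AIMoveTo with a blackboard radius, reporting success or failure.
; Tick records the enemy's last known location and refreshes the target, stopping and failing if it changes or the pawn is stunned.
; A walking pawn switches to running when farther than the blackboard strafe distance.
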(event EventReceiveExecuteAI
  (params (OwnerController :type AI%20Controller%20Object%20Reference) (ControlledPawn :type Pawn%20Object%20Reference))
  (Variables|Default|SetController OwnerController)
  (Variables|Default|SetDistanceFromTargetToStrafeVal (Class|BTFunctionLibrary|GetBlackboardValueasFloat (Variables|Default|GetDistanceFromActorToStrafe)))
  (Utilities|FlowControl|Sequence
    (:then_0
      (bind _asbp_ai_main (Utilities|Casting|CastToBP_AI_Main ControlledPawn))
      (bind _output_get (Variables|Default|SetAIPawn _asbp_ai_main))
      (Variables|/Script/Engine.CharacterMovementComponent|SetbOrientRotationToMovement (Variables|/Script/Engine.Character|GetCharacterMovement _output_get) true))
    (:then_1
      (Variables|Default|SetEnemyRef (AI|BehaviorTree|GetBlackboardValueasActor (Variables|Default|GetEnemy)))
      (Utilities|IsValid (Variables|Default|GetEnemyRef)
        (:Is%20Valid
          (AI|AIMoveTo (Variables|Default|GetController) "0, 0, 0" (Variables|Default|GetEnemyRef) (Class|BTFunctionLibrary|GetBlackboardValueasFloat (Variables|Default|GetRaduis)) "Default" "Default" true false
            (:OnRequestFailed
              (AI|BehaviorTree|FinishExecute false))
            (:OnMoveFinished
              (AI|BehaviorTree|FinishExecute true))))
        (:Is%20Not%20Valid
          (AI|BehaviorTree|FinishExecute false))))))

(event EventTick
  (params (OwnerActor :type Actor%20Object%20Reference) (DeltaSeconds :type Float%20%28single-precision%29))
  (bind _enemyref (Variables|Default|GetEnemyRef))
  (bind _aipawn (Variables|Default|GetAIPawn))
  (Utilities|IsValid _enemyref
    (:Is%20Valid
      (AI|BehaviorTree|SetBlackboardValueasVector (Variables|Default|GetLastKnownLoc) (Transformation|GetActorLocation _enemyref))
      (bind _output_get (Default|SetNewTarget (Variables|Default|GetAIPawn)))
      (if (or (!= _output_get (Variables|Default|GetEnemyRef)) (Default|IsStunned? (Variables|Default|GetAIPawn)))
        (AI|Navigation|StopMovement (Variables|Default|GetController))
        (AI|BehaviorTree|FinishExecute false)
        (elif (Default|IsWalking? _aipawn)
          (if (> (Math|Vector|VectorLength (- (Transformation|GetActorLocation _aipawn) (Transformation|GetActorLocation (Variables|Default|GetEnemyRef)))) (Variables|Default|GetDistanceFromTargetToStrafeVal))
            (Default|SetWalkRun (Variables|Default|GetAIPawn) false false)))))))