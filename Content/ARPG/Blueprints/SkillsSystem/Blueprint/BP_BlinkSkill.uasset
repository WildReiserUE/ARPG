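; Blink skill that, on the server, teleports a player-owned pawn to the cursor in top-down mode or forward otherwise, capped at a maximum range.
; TryFindLocation sphere-traces for capsule clearance, retrying at random offsets around the first blocking actor.
; Top-down destinations also require ground that projects onto the navmesh.
; After a top-down blink, it stops movement and messages the controller with the new transform.
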(event EventBeginPlay
  (bind _pawnowner (Variables|Default|GetPawnOwner))
  (bind _pawnowner_2 (Variables|Default|GetPawnOwner))
  ;[1 1 1] Blink skill
  (|CallParentFunction)
  (Networking|SwitchHasAuthority
    (:Authority
      (if (not (Variables|Default|GetOwnerIsAI))
        (bind _result (Class|BPCharacterInventoryInterface|CharacterIsTopDown(Message) _pawnowner))
        (bind _output_get (Variables|Default|SetIsTopDown _result))
        (if _output_get
          _
          (else
            (Variables|Default|SetCursorWorldLoc (+ (Transformation|GetActorLocation _pawnowner) (* (Transformation|GetActorForwardVector _pawnowner) 7e+02)))))
        (bind (_height _radius) (Class|ITSkillEffects|SkillGetCapsuleSize(Message) (Variables|Default|GetPawnOwner)))
        (bind _output_get_2 (Variables|Default|SetLocationToUse (Math|Vector|SelectVector (+ (* (Math|Rotator|GetRotationXVector (Math|Conversions|RotationFromXVector (- (Transformation|GetActorLocation _pawnowner) (Variables|Default|GetCursorWorldLoc)))) -1e+03) (Transformation|GetActorLocation (Variables|Default|GetPawnOwner))) (Variables|Default|GetCursorWorldLoc) (> (Math|Vector|VectorLength (- (Transformation|GetActorLocation _pawnowner) (Variables|Default|GetCursorWorldLoc))) 1e+03))))
        (bind (_success _location) (CallFunction|TryFindLocation _output_get_2 _height _radius))
        (if _success
          (Transformation|SetActorLocationAndRotation _pawnowner_2 _location (Math|Rotator|MakeRotator 0.0 0.0 (.yaw (Math|Rotator|FindLookatRotation (Transformation|GetActorLocation) _location))) false true)
          (if (Variables|Default|GetIsTopDown)
            (Components|Movement|StopMovementImmediately (Actor|GetComponentbyClass _pawnowner_2 "/Script/Engine.CharacterMovementComponent"))
            (bind _controller (Class|BPCharacterInventoryInterface|CharacterGetControllerRef(Message) (Variables|Default|GetPawnOwner)))
            (Class|BPARPGControllerInterface|ControlleronAbilityTeleport(Message) _controller _location (Math|Rotator|MakeRotator 0.0 0.0 (.yaw (Math|Rotator|FindLookatRotation (Transformation|GetActorLocation) _location))))))))))

(fn ConstructionScript
  (|CallParentFunction))

(fn TryFindLocation
  (params (InitialLoc :type Vector) (Height :type Float%20%28single-precision%29) (Radius :type Float%20%28single-precision%29))
  (bind _output_get (LocalVariables|SetStart (+ InitialLoc (Math|Vector|MakeVector 0.0 0.0 (/ Height 2.0)))))
  (bind _output_get_2 (LocalVariables|SetEnd (+ _output_get (Math|Vector|MakeVector 0.0 0.0 Height))))
  (LocalVariables|SetOrigStart _output_get)
  (LocalVariables|SetOrigEnd _output_get_2)
  (for _index (range 0 100)
    (bind (_outhit _returnvalue) (Collision|SphereTraceByChannel (LocalVariables|GetStart) (LocalVariables|GetEnd) Radius "TraceTypeQuery3" false (Utilities|Array|MakeArray (Variables|Default|GetPawnOwner)) "None"))
    (if _returnvalue
      (Utilities|FlowControl|Sequence
        (:then_0
          (if (and (Utilities|IsValid (.HitActor (Collision|BreakHitResult _outhit))) (not (LocalVariables|GetFoundActor)))
            (LocalVariables|SetFoundActor true)
            (LocalVariables|SetOrigStart (Transformation|GetActorLocation (.HitActor (Collision|BreakHitResult _outhit))))
            (LocalVariables|SetOrigEnd (+ (Transformation|GetActorLocation (.HitActor (Collision|BreakHitResult _outhit))) (Math|Vector|MakeVector 0.0 0.0 Height)))))
        (:then_1
          (LocalVariables|SetRandomX (Math|Random|RandomFloatinRange -1e+02 1e+02))
          (LocalVariables|SetRandomY (Math|Random|RandomFloatinRange -1e+02 1e+02))
          (LocalVariables|SetStart (+ (LocalVariables|GetOrigStart) (Math|Vector|MakeVector (LocalVariables|GetRandomX) (LocalVariables|GetRandomY) 0.0)))
          (LocalVariables|SetEnd (+ (LocalVariables|GetOrigEnd) (Math|Vector|MakeVector (LocalVariables|GetRandomX) (LocalVariables|GetRandomY) 0.0)))))
      (elif (Variables|Default|GetIsTopDown)
        (bind (_outhit_2 _returnvalue_2) (Collision|LineTraceByChannel (.TraceStart (Collision|BreakHitResult _outhit)) (+ (.TraceStart (Collision|BreakHitResult _outhit)) "0, 0,-500.000000") "TraceTypeQuery3" false (Utilities|Array|MakeArray (Variables|Default|GetPawnOwner)) "None"))
        (if _returnvalue_2
          (if (.ReturnValue (AI|Navigation|ProjectPointtoNavigation (.Location (Collision|BreakHitResult _outhit_2)) 0 0 "0, 0, 0"))
            (return true (+ (.Location (Collision|BreakHitResult _outhit_2)) (Math|Vector|MakeVector 0.0 0.0 (/ Height 2.0))))))
        (else
          (return true (+ (.TraceStart (Collision|BreakHitResult _outhit)) (Math|Vector|MakeVector 0.0 0.0 (* (/ Height 2.0) -1.0))))))))
  (return false "0, 0, 0"))