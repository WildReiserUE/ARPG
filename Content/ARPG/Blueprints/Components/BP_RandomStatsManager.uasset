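; BP_RandomStatsManager rolls random stats for items from an SJigItemRandomStats definition.
; GetRandomStats walks the roll list in order, clamps max to min, adds stats that pass their percent chance and stops at MaxStats.
; AdjustGetRandomRange rolls values truncated to two decimals, retrying up to 100 times so range stats get distinct min and max.
; Integer stats compare truncated values during those retries and are stored truncated.
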(fn GetRandomStats
  (params (S_JigItemRandomStats :type S%20Jig%20Item%20Random%20Stats%20Structure%20%28by%20ref%29))
  (bind (_rollstats _maxstats) (Utilities|Struct|BreakS_JigItemRandomStats S_JigItemRandomStats))
  ;[1 1 1] Generate random stats
  (Utilities|FlowControl|Sequence
    (:then_0
      (for _array_element _rollstats
        (bind _output_get (LocalVariables|SetCurrentVal _array_element))
        (Utilities|FlowControl|Sequence
          (:then_0
            (if (< (.MaxValue (Utilities|Struct|BreakS_RandomStat _output_get)) (.MinValue (Utilities|Struct|BreakS_RandomStat _output_get)))
              (Utilities|Struct|SetmembersinS_RandomStat (LocalVariables|GetCurrentVal) (.MinValue (Utilities|Struct|BreakS_RandomStat _output_get)))))
          (:then_1
            (if (<= (Math|Random|RandomFloatinRange 0.0 1e+02) (.Chance (Utilities|Struct|BreakS_RandomStat _output_get)))
              (bind (_randommin _randommax) (CallFunction|AdjustGetRandomRange (.MinValue (Utilities|Struct|BreakS_RandomStat _output_get)) (.MaxValue (Utilities|Struct|BreakS_RandomStat _output_get)) (.IsRangeStat? (Utilities|Struct|BreakS_RandomStat _output_get)) (.ResultIsInteger? (Utilities|Struct|BreakS_RandomStat _output_get))))
              (LocalVariables|SetRandomMin _randommin)
              (LocalVariables|SetRandomMax _randommax)
              (bind _returnvalue (Utilities|Array|Add (LocalVariables|GetStats) (Utilities|Struct|MakeItemStats (.Stat (Utilities|Struct|BreakS_RandomStat _output_get)) (LocalVariables|GetRandomMin) (LocalVariables|GetRandomMax))))
              (Utilities|FlowControl|Sequence
                (:then_0
                  (if (.ResultIsInteger? (Utilities|Struct|BreakS_RandomStat _output_get))
                    (Utilities|Struct|SetmembersinItemStats (Utilities|Array|Get(acopy) (LocalVariables|GetStats) _returnvalue) (Math|Conversions|ToFloat(Integer) (Math|Float|Truncate (.MinValue (Utilities|Struct|BreakItemStats (Utilities|Array|Get(acopy) (LocalVariables|GetStats) _returnvalue))))) (Math|Conversions|ToFloat(Integer) (Math|Float|Truncate (.MaxValue (Utilities|Struct|BreakItemStats (Utilities|Array|Get(acopy) (LocalVariables|GetStats) _returnvalue))))))))
                (:then_1
                  (bind _result (Math|Integer|IncrementInt (LocalVariables|GetTotalStats))
                    (:%20%20
                      (if (== _result _maxstats)
                        (return (LocalVariables|GetStats))))))))))))
    (:then_1
      (return (LocalVariables|GetStats)))))

(fn AdjustFloat
  (params (FloatVal :type Float%20%28single-precision%29))
  (return (/ (Math|Conversions|ToFloat(Integer) (Math|Float|Truncate (* 100 FloatVal))) 1e+02)))

(fn AdjustGetRandomRange
  (params (Min :type Float%20%28single-precision%29) (Max :type Float%20%28single-precision%29) (IsRange :type Boolean) (Integer :type Boolean))
  (bind _returnvalue (== Max 0.0))
  (bind _returnvalue_2 (Math|Float|SelectFloat Min Max _returnvalue))
  (bind _returnvalue_3 (Math|Random|RandomFloatinRange Min _returnvalue_2))
  (bind _returnvalue_4 (CallFunction|AdjustFloat _returnvalue_3))
  ;[1 1 1] Avoid getting the same value in both min amd max for range stats
  (Utilities|FlowControl|Sequence
    (:then_0
      (if (and (!= Min Max) IsRange)
        (for _index (range 0 99)
          (bind _output_get (LocalVariables|SetFinalMin (CallFunction|AdjustFloat (Math|Random|RandomFloatinRange Min Max))))
          (LocalVariables|SetFinalMax (CallFunction|AdjustFloat (Math|Random|RandomFloatinRange _output_get Max)))
          (if Integer
            (if (!= (Math|Float|Truncate (LocalVariables|GetFinalMin)) (Math|Float|Truncate (LocalVariables|GetFinalMax)))
              (return (LocalVariables|GetFinalMin) (LocalVariables|GetFinalMax)))
            (elif (!= (LocalVariables|GetFinalMin) (LocalVariables|GetFinalMax))
              (return (LocalVariables|GetFinalMin) (LocalVariables|GetFinalMax)))))
        (else
          (return _returnvalue_4 _returnvalue_4))))
    (:then_1
      (return (LocalVariables|GetFinalMin) (LocalVariables|GetFinalMax)))))