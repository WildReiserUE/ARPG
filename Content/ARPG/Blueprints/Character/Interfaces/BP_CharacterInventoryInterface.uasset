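; Blueprint interface that lets other systems talk to an ARPG player character, mainly around inventory, equipment and stats.
; It declares calls for equipping and swapping gear by slot, item and mod events, actionbar input, health and mana restoration, and stat and attribute access.
; It also covers click-to-move, camera zoom and rotation, respawn, controller ownership, party leadership and god mode.
; Functions are empty declarations, so implementers supply all behaviour.
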(fn GetEquipmentMeshbySlot
  (params (Slot :type EquipmentSlots%20Enum :default "NewEnumerator12"))
  (return 0))

(fn EquipItembySlot
  (params (ToSlot :type EquipmentSlots%20Enum :default "NewEnumerator12") (EquipmentClass :type BP%20Main%20Equipment%20Class%20Reference) (ToSocket :type Name) (LocalServer? :type Boolean) (ItemID :type Name) (DtRef :type Data%20Table%20Object%20Reference))
  (return false))

(fn SwapPrimarySecondary
  (params (PrimarySocket :type Name) (SecondarySocket :type Name) (Slot :type EquipmentSlots%20Enum :default "NewEnumerator12"))
  (return false))

(fn CharacterGetInventoryComponent
  (return 0))

(fn GetPlayerstats
  (return "" 0 "" 0))

(fn SetPlayerStats
  (params (Stats :type S%20Player%20Stats%20Structure) (StatsAllocation :type Integer) (PlayerName :type String) (AllocatorTracker :type S%20Stats%20Allocation%20Tracker%20Structure) (Effects :type Map%20of%20Integers%20to%20Structs) (EffectTracker :type Map%20of%20Integers%20to%20Structs))
  (return false))

(fn ActionbarKeyPress
  (params (Actionbar :type E_ActionbarSlots%20Enum :default "NewEnumerator4") (InvComp :type BP%20Inventory%20Component%20Object%20Reference) (TargetRot :type Rotator) (TargetRef :type Actor%20Object%20Reference) (LocationUnderCursor :type Vector))
  (return false))

(fn JigMovetoLocation
  (params (Location :type Vector)))

(fn JigMovetoActor
  (params (ActorRef :type Actor%20Object%20Reference) (CustomRange :type Float%20%28single-precision%29)))

(fn JigZoomOut)

(fn JigZoomin)

(fn JigRespawn
  (return false))

(fn SetControllerOwner
  (params (ControllerRef :type Player%20Controller%20Object%20Reference))
  (return))

(fn JigonModInstalled
  (params (Info :type Container%20Items%20Structure) (HandleRep :type Boolean))
  (return false))

(fn JigonModRemoved
  (params (Info :type Container%20Items%20Structure) (HandleRep :type Boolean))
  (return false))

(fn JigRestoreHealth
  (params (Value :type Float%20%28single-precision%29) (FromSkill :type Boolean))
  (return false))

(fn JigRestoreMana
  (params (Value :type Float%20%28single-precision%29))
  (return false))

(fn JigonItemEquipped
  (params (Info :type F%20Item%20Info%20Structure) (Items :type Array%20of%20Container%20Items%20Structures) (HandleRep :type Boolean))
  (return false))

(fn JigonItemUnEquipped
  (params (Info :type F%20Item%20Info%20Structure) (Items :type Array%20of%20Container%20Items%20Structures) (HandleRep :type Boolean))
  (return false))

(fn JigGetPlayerLevel
  (return 0))

(fn JigTPPLeftMouseClick
  (params (TargetAtCursor :type Actor%20Object%20Reference))
  (return false))

(fn SetAllocatedAttributes
  (params (STR :type Integer) (DEX :type Integer) (INT :type Integer) (END :type Integer))
  (return false))

(fn JigonItemConsumed
  (params (ItemInfo :type F%20Item%20Info%20Structure))
  (return false))

(fn GetLocalCharacter
  (return 0))

(fn SetLocalPlayer
  (return))

(fn GetReplicatedStats
  (return ""))

(fn CharacterGetControllerRef
  (return 0))

(fn CharacterIsPartyLeader
  (return false))

(fn CharacterSetIsPartyLeader
  (params (Value :type Boolean))
  (return false))

(fn CharacterIsTopDown
  (return false))

(fn CharacterSetGodMode
  (params (GodMode :type Boolean))
  (return false))

(fn AddSpringArmRotation
  (params (Rotation :type Rotator) (Local? :type Boolean))
  (return false))